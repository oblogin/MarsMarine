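; Player marine pawn for Mars Marine, with world-axis movement, twin-stick style aiming, rifle fire and a HUD.
; Each tick it sets control rotation from thumbstick direction or smoothed mouse velocity, using deadzones and the last pressed key's device type.
; Fire input toggles a particle system and looping sound, with an end sound on release.
; Each press also subtracts Health and recolors the dynamic material's emissive and glass from red-green health values.
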(event EventBeginPlay
  (bind _returnvalue (UserInterface|CreateWidget "/Game/MarsMarine/HUD/W_PlayerHUD.W_PlayerHUD_C" 0 self))
  (bind _output_get (Variables|Default|SetPlayerHUD _returnvalue))
  (UserInterface|Viewport|AddtoViewport _output_get 0)
  (bind _returnvalue_2 (Rendering|Material|CreateDynamicMaterialInstance (Variables|Character|GetMesh) 0 0 "None" :!class /Script/Engine.PrimitiveComponent))
  (Variables|Default|SetMarrineMaterial _returnvalue_2))

(event Collision|EventActorBeginOverlap
  (params (OtherActor :type Actor%20Object%20Reference)))

(event EventTick
  (params (DeltaSeconds :type Float%20%28single-precision%29))
  (CallFunction|UpdatePlayerAim))

(event Input|ActionEvents|InputActionFireWEapon
  (params (Key :type Key%20Structure :default "None"))
  (bind _linearcolor (CallFunction|GetHealthBarColor))
  (:Pressed
    (CallFunction|StartFiringWeapon)
    (Variables|Default|SetHealth (- (Variables|Default|GetHealth) 5.0))
    (Rendering|Material|SetVectorParameterValue (Variables|Default|GetMarrineMaterial) "Emissive Color" _linearcolor :!class /Script/Engine.MaterialInstanceDynamic)
    (Rendering|Material|SetVectorParameterValue (Variables|Default|GetMarrineMaterial) "Glass Color" _linearcolor :!class /Script/Engine.MaterialInstanceDynamic))
  (:Released
    (CallFunction|StopFiringWeapon)))

(event Input|AxisEvents|InputAxisMoveRight
  (params (AxisValue :type Float%20%28single-precision%29))
  (Pawn|Input|AddMovementInput "0.000000,1.000000, 0" AxisValue false))

(event Input|AxisEvents|InputAxisMoveForward
  (params (AxisValue :type Float%20%28single-precision%29))
  (Pawn|Input|AddMovementInput "1.000000, 0, 0" AxisValue false))

(event Input|KeyboardEvents|AnyKey
  (params (Key :type Key%20Structure :default "None"))
  (:Pressed
    (Variables|Default|SetIsGamepadActive (Class|KismetInputLibrary|KeyIsGamepadKey Key))))

(fn ConstructionScript)

(fn UpdatePlayerAim
  (if (Variables|Default|GetIsGamepadActive)
    (ThumbstickInput|UpdateThumbstickAim)
    (else
      (MouseInput|UpdateMouseAim))))

(fn IsThumbstickAboveDeadzone
  (return (> (Math|Vector2D|Vector2DLength (Math|Vector2D|MakeVector2D (Input|AxisValues|GetThumbstickAimUp) (Input|AxisValues|GetThumbstickAimRight))) (LocalVariables|GetThumbstickDeadzone))))

(fn UpdateMouseAim
  (if (MouseInput|IsMouseAboveDeadzone)
    (Pawn|SetControlRotation (Game|GetPlayerController 0) (MouseInput|GetMouseAimDirection))))

(fn IsMouseAboveDeadzone
  (return (> (Math|Vector2D|Vector2DLength (MouseInput|GetMouseVelocity)) (LocalVariables|GetMouse%20Deadzone))))

(fn GetMouseVelocity
  (bind _returnvalue (Game|GetPlayerController 0))
  (bind (_deltax _deltay) (Class|PlayerController|GetInputMouseDelta _returnvalue))
  (return (/ (Math|Vector2D|MakeVector2D _deltax _deltay) (Utilities|Time|GetWorldDeltaSeconds))))

(fn GetMouseAimDirection
  (bind _returnvalue (MouseInput|GetMouseVelocity))
  (return (Math|Interpolation|RInterpTo (Pawn|GetControlRotation (Game|GetPlayerController 0) :!class /Script/Engine.Controller) (Math|Rotator|MakeRotator 0.0 0.0 (Class|KismetMathLibrary|DegAtan2 (.x _returnvalue) (.y _returnvalue))) (Utilities|Time|GetWorldDeltaSeconds) (LocalVariables|GetMouse%20Smoothing%20Strength))))

(fn UpdateThumbstickAim
  (if (ThumbstickInput|IsThumbstickAboveDeadzone)
    (Pawn|SetControlRotation (Game|GetPlayerController 0) (ThumbstickInput|GetThumbstickAimDirection))))

(fn GetThumbstickAimDirection
  (return (Math|Rotator|MakeRotator 0.0 0.0 (Class|KismetMathLibrary|DegAtan2 (Input|AxisValues|GetThumbstickAimRight) (Input|AxisValues|GetThumbstickAimUp)))))

(fn StartFiringWeapon
  (Components|Activation|Activate (Variables|Default|GetParticleSystem) false)
  (bind _returnvalue (Audio|SpawnSound2D "/Game/Sounds/Weapon_AssaultRifle/Stereo/RifleFireLoop_Cue.RifleFireLoop_Cue" 1.0 1.0 0.0 0 false false))
  (Variables|Default|SetWeaponFireSound _returnvalue))

(fn StopFiringWeapon
  (Components|Activation|Deactivate (Variables|Default|GetParticleSystem))
  (Audio|Components|Audio|Stop (Variables|Default|GetWeaponFireSound))
  (Audio|SpawnSound2D "/Game/Sounds/Weapon_AssaultRifle/Stereo/RifleFireEnd_Cue.RifleFireEnd_Cue" 1.0 1.0 0.0 0))

(fn GetHealthBarColor
  (bind _health (Variables|Default|GetHealth))
  (bind _returnvalue (/ _health 1e+02))
  (bind _returnvalue_2 (- 1.0 _returnvalue))
  (bind _returnvalue_3 (* _returnvalue_2 1e+02))
  (Development|PrintString (Utilities|String|ToString(Float) _returnvalue_3))
  (return (Utilities|Struct|MakeLinearColor _returnvalue_3 (* _returnvalue 1e+02) 0.0 1.0)))