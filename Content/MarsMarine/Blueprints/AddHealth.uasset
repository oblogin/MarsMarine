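; AddHealth is a health pickup actor for the marine character.
; On BeginPlay it rolls a random integer heal amount between its minimum and maximum variables.
; When a BP_Marine overlaps it, it adds that amount directly to the marine's Health, with no clamp in this Blueprint, then destroys itself.
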(event Collision|EventActorBeginOverlap
  (params (OtherActor :type Actor%20Object%20Reference))
  (bind _asbp_marine (Utilities|Casting|CastToBP_Marine OtherActor))
  (Variables|/Game/MarsMarine/Blueprints/Pawns/BP_Marine.BP_Marine_C|SetHealth _asbp_marine (+ (Variables|/Game/MarsMarine/Blueprints/Pawns/BP_Marine.BP_Marine_C|GetHealth _asbp_marine) (Math|Conversions|ToFloat(Integer) (Variables|Default|GetAddHealth))))
  (Actor|DestroyActor))

(event EventBeginPlay
  (Variables|Default|SetAddHealth (Math|Random|RandomIntegerinRange (Variables|Default|GetMinHealt) (Variables|Default|GetMaxHealt))))

(fn ConstructionScript)