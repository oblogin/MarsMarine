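; BP_SpawnArea is a placeable area that scatters resource actors across the landscape when play begins.
; SpawnResource makes MinCount attempts, box-tracing downward on the Visibility channel at random points within the actor's XY bounds.
; It spawns ActorOfSpawn at the impact point only when the hit actor is a Landscape.
; Failed attempts are not retried, so the area can yield fewer than MinCount actors.
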(event EventBeginPlay
  (CallFunction|SpawnResource))

(event Collision|EventActorBeginOverlap
  (params (OtherActor :type Actor%20Object%20Reference)))

(event EventTick
  (params (DeltaSeconds :type Float%20%28single-precision%29)))

(fn ConstructionScript)

(fn SpawnResource
  (bind (_origin _boxextent) (Collision|GetActorBounds false false))
  (bind _z (Math|Vector|BreakVector _origin))
  (bind (_x _y) (Math|Vector|BreakVector _boxextent))
  (bind _returnvalue (* _y 2.0))
  (bind _returnvalue_2 (* _x 2.0))
  (bind _returnvalue_3 (- _y _returnvalue))
  (bind _returnvalue_4 (- _x _returnvalue_2))
  (bind _returnvalue_5 (Math|Random|RandomFloatinRange _returnvalue_3 _y))
  (bind _returnvalue_6 (Math|Random|RandomFloatinRange _returnvalue_4 _x))
  (bind _returnvalue_7 (Math|Vector|MakeVector _returnvalue_6 _returnvalue_5 _z))
  (bind _returnvalue_8 (+ _origin _returnvalue_7))
  (for _index (range 1 (Variables|Default|GetMinCount))
    (bind _outhit (Collision|BoxTraceByChannel (+ _returnvalue_8 "0, 0,1000.000000") (- _returnvalue_8 "0.0,0.0,200.000000") "25.000000,25.000000,25.000000" "0, 0, 0" "TraceTypeQuery1" false 0 "None" true "(R=1.000000,G=0.000000,B=0.000000,A=1.000000)" "(R=0.000000,G=1.000000,B=0.000000,A=1.000000)" 1.0))
    (if (== (Utilities|GetClass (.HitActor (Collision|BreakHitResult _outhit))) "/Script/Landscape.Landscape")
      (bind _returnvalue_9 (Game|SpawnActorfromClass (Variables|Default|GetActorOfSpawn) (Math|Conversions|ToTransform(Vector) (.ImpactPoint (Collision|BreakHitResult _outhit))) "Undefined" 0 0))
      (LocalVariables|SetSpawnActor _returnvalue_9))))