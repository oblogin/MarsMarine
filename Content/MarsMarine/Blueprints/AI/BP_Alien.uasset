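; Alien enemy AI that chases the Marine player and plays an attack montage in range, pausing movement.
; Point damage is reduced by Armor, doubled for BP_CritDamage, and shown as spawned combat text.
; Health scales with Endurance and drives a dynamic-material health bar, toggled by cursor hover.
; At zero health it stops, disables collision and increments the Marine's kills; DamagePlayer is defined but not called here.
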(event EventBeginPlay
  (bind _asbp_marine (Utilities|Casting|CastToBP_Marine (Game|GetPlayerCharacter 0)))
  (Variables|Default|SetRefMarine _asbp_marine)
  (Variables|Default|SetHealth (CallFunction|GetMaxHealth))
  (bind _returnvalue (Rendering|Material|CreateDynamicMaterialInstance (Variables|Default|GetHealthBar) 0 0 "None" :!class /Script/Engine.PrimitiveComponent))
  (Variables|Default|SetMaterialHeathBar _returnvalue)
  (CallFunction|UpdateHealthBar)
  (if (and (CallFunction|IsAlive) (Default|IsAlive (Variables|Default|GetRefMarine))) :!label _label
    (AI|AIMoveTo self "0, 0, 0" (Variables|Default|GetRefMarine) 5.0 true
      (:OnSuccess
        _)
      (:OnFail
        _))
    (Utilities|FlowControl|Delay 0.2)
    (goto _label)))

(event MouseInput|EventActorBeginCursorOver
  ;[1 1 1] Toggle Health Bar visibile
  (Rendering|SetVisibility (Variables|Default|GetHealthBar) true false))

(event EventTick
  (params (DeltaSeconds :type Float%20%28single-precision%29))
  (if (CallFunction|CanAttack)
    (Components|Activation|Deactivate (Variables|Character|GetCharacterMovement))
    (Animation|Montage|PlayMontage (Variables|Character|GetMesh) "/Game/Characters/Enemy_Great_Spider/Animations/AlienAttack.AlienAttack"
      (:then
        (if (not (Default|IsAlive (Variables|Default|GetRefMarine)))
          (CallFunction|KillAI)))
      (:OnCompleted
        (Components|Activation|Activate (Variables|Character|GetCharacterMovement) false)))))

(event MouseInput|EventActorEndCursorOver
  ;[1 1 1] Toggle Health Bar visibile
  (Rendering|SetVisibility (Variables|Default|GetHealthBar) false false))

(event Game|Damage|EventPointDamage
  (params (Damage :type Float%20%28single-precision%29) (DamageType :type Damage%20Type%20Object%20Reference) (HitLocation :type Vector :default "0, 0, 0") (HitNormal :type Vector :default "0, 0, 0") (HitComponent :type Primitive%20Component%20Object%20Reference) (BoneName :type Name :default "None") (ShotFromDirection :type Vector :default "0, 0, 0") (InstigatedBy :type Controller%20Object%20Reference) (DamageCauser :type Actor%20Object%20Reference) (HitInfo :type Hit%20Result%20Structure%20%28by%20ref%29))
  (bind _damagereceived (Combat|CalculateDamage Damage DamageType))
  (bind _health (CallFunction|DecreaseHealth _damagereceived))
  (HUD|CreateDamageWidget HitLocation _damagereceived DamageType)
  (CallFunction|UpdateHealthBar)
  (if (== _health 0.0)
    (CallFunction|KillAI)
    (Collision|SetActorEnableCollision false)
    (Default|IncreaseKills (Variables|Default|GetRefMarine))))

(fn ConstructionScript)

(fn IsWithinAttackRange
  (return (< (Transformation|GetDistanceTo (Game|GetPlayerCharacter 0)) (LocalVariables|GetAttackRange))))

(fn IsAttacking
  (return (Animation|Montage|MontageIsPlaying (Components|SkeletalMesh|GetAnimInstance (Variables|Character|GetMesh)) "/Game/Characters/Enemy_Great_Spider/Animations/AlienAttack.AlienAttack")))

(fn DamagePlayer
  (Game|Damage|ApplyDamage (Game|GetPlayerCharacter 0) (Variables|Default|GetDamage) 0 0))

(fn DecreaseHealth
  (params (Damage :type Float%20%28single-precision%29))
  (bind _output_get (Variables|Default|SetHealth (Math|Float|Clamp(Float) (- (Variables|Default|GetHealth) Damage) 0.0 (CallFunction|GetMaxHealth))))
  (return _output_get))

(fn IsAlive
  (return (not (Variables|Default|GetDeath))))

(fn KillAI
  (bind _charactermovement (Variables|Character|GetCharacterMovement))
  (Variables|Default|SetDeath true)
  (Components|Movement|StopMovementImmediately _charactermovement)
  (Components|Activation|Deactivate _charactermovement))

(fn CanAttack
  (return (Math|Boolean|ANDBoolean (CallFunction|IsWithinAttackRange) (not (CallFunction|IsAttacking)) (Default|IsAlive (Variables|Default|GetRefMarine)) (CallFunction|IsAlive))))

(fn GetMaxHealth
  (return (Math|Conversions|ToFloat(Integer) (* (Variables|Stats|GetEndurance) 10))))

(fn UpdateHealthBar
  (Rendering|Material|SetVectorParameterValue (Variables|Default|GetMaterialHeathBar) "Color" (Utilities|CalcHealthColor (Variables|Default|GetHealth) (CallFunction|GetMaxHealth)) :!class /Script/Engine.MaterialInstanceDynamic)
  (Rendering|Material|SetScalarParameterValue (Variables|Default|GetMaterialHeathBar) "Progress" (/ (Variables|Default|GetHealth) (CallFunction|GetMaxHealth)) :!class /Script/Engine.MaterialInstanceDynamic))

(fn MouseOffsetCamera)

(fn CreateDamageWidget
  (params (SpawnLocation :type Vector) (Damage :type Float%20%28single-precision%29) (DamageType :type Damage%20Type%20Object%20Reference))
  (Utilities|Casting|CastToBP_CritDamage DamageType
    (:then
      (Game|SpawnActorfromClass "/Game/MarsMarine/Blueprints/BP_CombatText.BP_CombatText_C" (Math|Transform|MakeTransform SpawnLocation "0, 0, 0" "1,1,1") "Undefined" 0 Damage true 0))
    (:CastFailed
      (Game|SpawnActorfromClass "/Game/MarsMarine/Blueprints/BP_CombatText.BP_CombatText_C" (Math|Transform|MakeTransform SpawnLocation "0, 0, 0" "1,1,1") "Undefined" 0 Damage false 0))))

(fn CalculateDamage
  (params (Damage :type Float%20%28single-precision%29) (NewParam :type Damage%20Type%20Object%20Reference))
  (bind _armor (Variables|Stats|GetArmor))
  (bind _returnvalue (Math|Conversions|ToFloat(Integer) _armor))
  (bind _returnvalue_2 (- Damage _returnvalue))
  (Utilities|Casting|CastToBP_CritDamage NewParam
    (:then
      (return (* _returnvalue_2 2.0)))
    (:CastFailed
      (return _returnvalue_2))))