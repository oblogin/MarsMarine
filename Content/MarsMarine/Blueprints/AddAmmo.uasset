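; AddAmmo is an ammo pickup actor that restocks the marine's ammunition.
; On BeginPlay it rolls a random amount between MinAmmo and MaxAmmo.
; When a BP_Marine overlaps it, it adds that amount directly to the marine's Ammo variable, then destroys itself.
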(event Collision|EventActorBeginOverlap
  (params (OtherActor :type Actor%20Object%20Reference))
  (bind _asbp_marine (Utilities|Casting|CastToBP_Marine OtherActor))
  (Variables|/Game/MarsMarine/Blueprints/Pawns/BP_Marine.BP_Marine_C|SetAmmo _asbp_marine (+ (Variables|/Game/MarsMarine/Blueprints/Pawns/BP_Marine.BP_Marine_C|GetAmmo _asbp_marine) (Variables|Default|GetAmmo)))
  (Actor|DestroyActor))

(event EventBeginPlay
  (Variables|Default|SetAmmo (Math|Random|RandomIntegerinRange (Variables|Default|GetMinAmmo) (Variables|Default|GetMaxAmmo))))

(fn ConstructionScript)