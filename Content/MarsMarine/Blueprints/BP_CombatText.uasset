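; BP_CombatText is a short-lived actor that shows floating damage numbers through a CombatWidget on its widget component.
; On BeginPlay it gets the widget, tints it red for critical hits and plays the combat text with the Damage value.
; It destroys itself after a brief delay.
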(event EventBeginPlay
  (bind _ascombat_widget (Utilities|Casting|CastToCombatWidget (UserInterface|GetUserWidgetObject (Variables|Default|GetCombatTextWidget))))
  (Variables|Default|SetAsCombatWidget _ascombat_widget)
  (if (Variables|Default|GetIsCritical)
    (Appearance|SetColorandOpacity (Variables|Default|GetAsCombatWidget) "(R=1.000000,G=0.000000,B=0.000000,A=1.000000)" :!class /Script/UMG.UserWidget))
  (Default|PlayCombatText (Variables|Default|GetAsCombatWidget) (Variables|Default|GetDamage))
  (Utilities|FlowControl|Delay 1.5)
  (Actor|DestroyActor))

(fn ConstructionScript)