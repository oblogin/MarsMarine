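; BP_WeaponMaster is the marine's base firearm, handling automatic fire, ammo clip and timed reload.
; Firing starts muzzle VFX and sound, then a looping timer runs line traces toward the cursor, with random spread scaled by distance, Perception and Accuracy.
; Hits apply point damage, using a crit damage type by chance, and spawn impact effects.
; An empty clip triggers a reload that updates the marine's progress widget, draws from its ammo and resumes firing.
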(event Custom|StartFiring
  (if (CallFunction|IsAmmoClip)
    (CallFunction|StartFiring)
    (else
      (CallFunction|ReloadAmmo))))

(event Custom|StopFiring
  (CallFunction|StopFiring))

(event Custom|ReloadAmmo
  (if (not (== (Variables|Default|GetAmmoСlip) (Variables|Default|GetMaxAmmoСlip)))
    (CallFunction|StopFiring)
    (Variables|Default|SetStartReloadTime (Utilities|Time|GetGameTimeinSeconds))
    (Rendering|SetVisibility (Variables|/Game/MarsMarine/Blueprints/Pawns/BP_Marine.BP_Marine_C|GetReloadWidget (Variables|Ref|GetAsMarine)) true false)
    (if (< (Utilities|Time|GetGameTimeinSeconds) (+ (Variables|Default|GetStartReloadTime) (Variables|Default|GetReloadTime))) :!label _label
      (Variables|/Game/MarsMarine/HUD/W_RealoadWidget.W_RealoadWidget_C|SetProgress (Variables|/Game/MarsMarine/Blueprints/Pawns/BP_Marine.BP_Marine_C|GetRefRealoadWidget (Variables|Ref|GetAsMarine)) (Math|Float|Lerp 0.0 1.0 (CallFunction|GetReloadProgress)))
      (Utilities|FlowControl|Delay 0.1)
      (goto _label)
      (else
        (Rendering|SetVisibility (Variables|/Game/MarsMarine/Blueprints/Pawns/BP_Marine.BP_Marine_C|GetReloadWidget (Variables|Ref|GetAsMarine)) false false)
        (if (>= (Variables|/Game/MarsMarine/Blueprints/Pawns/BP_Marine.BP_Marine_C|GetAmmo (Variables|Ref|GetAsMarine)) (CallFunction|CountAmmoReloading))
          (Variables|/Game/MarsMarine/Blueprints/Pawns/BP_Marine.BP_Marine_C|SetAmmo (Variables|Ref|GetAsMarine) (- (Variables|/Game/MarsMarine/Blueprints/Pawns/BP_Marine.BP_Marine_C|GetAmmo (Variables|Ref|GetAsMarine)) (CallFunction|CountAmmoReloading)))
          (Variables|Default|SetAmmoСlip (+ (CallFunction|CountAmmoReloading) (Variables|Default|GetAmmoСlip)))
          (else
            (Variables|Default|SetAmmoСlip (Variables|/Game/MarsMarine/Blueprints/Pawns/BP_Marine.BP_Marine_C|GetAmmo (Variables|Ref|GetAsMarine)))
            (Variables|/Game/MarsMarine/Blueprints/Pawns/BP_Marine.BP_Marine_C|SetAmmo (Variables|Ref|GetAsMarine) 0)))
        (if (Variables|Default|GetIsFiring)
          (CallFunction|StartFiring))))))

(event EventBeginPlay
  (bind _asbp_marine (Utilities|Casting|CastToBP_Marine (Components|GetOwner)))
  (Variables|Ref|SetAsMarine _asbp_marine)
  (bind _returnvalue (Effects|SpawnEmitterAttached (Variables|Ref|GetFireVFX) self "FlashSocket" "0, 0,0.000000" "0, 0, 0" "1.000000,1.000000,1.000000" "KeepRelativeOffset" false "None" false))
  (Variables|Default|SetRefFireVFX _returnvalue))

(event EventTick
  (params (DeltaSeconds :type Float%20%28single-precision%29)))

(fn WeaponeTrace
  (bind _returnvalue (Game|GetPlayerController 0))
  (bind _returnvalue_2 (Transformation|GetWorldLocation))
  (bind _accuracy (Variables|Default|GetAccuracy))
  (bind _asmarine (Variables|Ref|GetAsMarine))
  (bind _hitresult (Game|Player|GetHitResultUnderCursorbyChannel _returnvalue "TraceTypeQuery1" true))
  (bind _perception (Variables|/Game/MarsMarine/Blueprints/Pawns/BP_Marine.BP_Marine_C|GetPerception _asmarine))
  (bind _location (Collision|BreakHitResult _hitresult))
  (bind _returnvalue_3 (* _perception 0.2))
  (bind _returnvalue_4 (- _returnvalue_2 _location))
  (bind _returnvalue_5 (+ _returnvalue_3 _accuracy))
  (bind _returnvalue_6 (Math|Vector|VectorLength _returnvalue_4))
  (bind _returnvalue_7 (/ _returnvalue_6 _returnvalue_5))
  (if (CallFunction|IsAmmoClip)
    (Math|Integer|DecrementInt (Variables|Default|GetAmmoСlip)
      (:%20%20
        (bind (_outhit _returnvalue_8) (Collision|LineTraceByChannel (Transformation|GetWorldLocation) (* (- (+ _location (Utilities|MakeRandomVector (* _returnvalue_7 -1.0) _returnvalue_7)) (Transformation|GetWorldLocation)) 1e+03) "TraceTypeQuery1" true 0 "None"))
        (if _returnvalue_8
          (Game|Damage|ApplyPointDamage (.HitActor (Collision|BreakHitResult _outhit)) (Variables|Default|GetBase%20Damage) (.TraceStart (Collision|BreakHitResult _outhit)) _outhit 0 0 (CallFunction|IsCrit))
          (Effects|SpawnEmitteratLocation "/Game/Effects/Weapons/Impacts/P_CreatureImpact.P_CreatureImpact" (.Location (Collision|BreakHitResult _outhit)) (Math|Conversions|RotationFromXVector (.Normal (Collision|BreakHitResult _outhit)))))))
    (else
      (CallFunction|ReloadAmmo))))

(fn StartFiring
  (Variables|Default|SetIsFiring true)
  (Components|Activation|Activate (Variables|Default|GetRefFireVFX) false)
  (bind _returnvalue (Audio|SpawnSound2D (Variables|Settings|GetFireSound) 1.0 1.0 0.0 0 false false))
  (Variables|Default|SetRefFireSound _returnvalue)
  (CallFunction|WeaponeTrace)
  (Utilities|Time|SetTimerbyFunctionName 0 "Weapone Trace" (/ 1.0 (Variables|Default|GetFire%20Rate)) true))

(fn StopFiring
  (bind _reffiresound (Variables|Default|GetRefFireSound))
  (Variables|Default|SetIsFiring false)
  (Components|Activation|Deactivate (Variables|Default|GetRefFireVFX))
  (Utilities|IsValid _reffiresound
    (:Is%20Valid
      (Audio|Components|Audio|Stop _reffiresound)
      (Utilities|Time|ClearTimerbyFunctionName 0 "Weapone Trace")
      (if (Default|IsAlive (Variables|Ref|GetAsMarine))
        (Audio|SpawnSound2D "/Game/Sounds/Weapon_AssaultRifle/Stereo/RifleFireEnd_Cue.RifleFireEnd_Cue" 1.0 1.0 0.0 0)))))

(fn IsAmmoClip
  (return (> (Variables|Default|GetAmmoСlip) 0)))

(fn IsCrit
  (if (<= (Math|Random|RandomIntegerinRange 0 100) (Variables|Default|GetCritChance))
    (return "/Game/MarsMarine/Blueprints/BP_CritDamage.BP_CritDamage_C")
    (else
      (return 0))))

(fn GetReloadProgress
  (return (/ (- (Utilities|Time|GetGameTimeinSeconds) (Variables|Default|GetStartReloadTime)) (Variables|Default|GetReloadTime))))

(fn CountAmmoReloading
  (return (- (Variables|Default|GetMaxAmmoСlip) (Variables|Default|GetAmmoСlip))))